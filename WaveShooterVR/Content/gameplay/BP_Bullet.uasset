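; BP_Bullet is a projectile actor that flies straight ahead and destroys itself on contact.
; Each tick it moves the Bullet component along the actor's forward vector at MovementSpeed, scaled by delta time, without sweeping or a projectile movement component.
; When the Bullet component begins an overlap, it prints the other actor's name and destroys the actor, applying no damage.
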(event `self.ReceiveTick`
  (params (DeltaSeconds :type "Float (single-precision)"))
  ;[1 1 1] move bullet forward
  (`SceneComponent.K2_AddWorldOffset` (`self.Bullet`) (* (* (`self.GetActorForwardVector`) (`self.MovementSpeed`)) (`GameplayStatics.GetWorldDeltaSeconds`)) false false))

(event `self.Bullet.OnComponentBeginOverlap`
  (params (OverlappedComponent :type "PrimitiveComponent Object Reference") (OtherActor :type "Actor Object Reference") (OtherComp :type "PrimitiveComponent Object Reference") (OtherBodyIndex :type Integer) (bFromSweep :type Boolean) (SweepResult :type "HitResult Structure (by ref)"))
  ;[1 1 1] log overlapped actor and destroy bullet
  (`KismetSystemLibrary.PrintString` (`KismetSystemLibrary.GetDisplayName` OtherActor))
  (`self.K2_DestroyActor`))

(fn `UserConstructionScript`)