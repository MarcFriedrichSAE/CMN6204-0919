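; Projectile actor that flies straight along its forward vector and damages characters on the opposing side.
; Tick moves the Bullet component by MovementSpeed scaled by delta time, without sweeping.
; On overlap, actor tags and the Origin string decide the hit: player shots hurt BP_Enemy, enemy shots deal lighter damage to BP_Friend.
; A sequence then destroys the bullet on any overlap, whether or not damage was dealt.
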(event `self.ReceiveTick`
  (params (DeltaSeconds :type "Float (single-precision)"))
  ;[1 1 1] move bullet forward
  (`SceneComponent.K2_AddWorldOffset` (`self.Bullet`) (* (* (`self.GetActorForwardVector`) (`self.MovementSpeed`)) (`GameplayStatics.GetWorldDeltaSeconds`)) false false))

(event `self.Bullet.OnComponentBeginOverlap`
  (params (OverlappedComponent :type "PrimitiveComponent Object Reference") (OtherActor :type "Actor Object Reference") (OtherComp :type "PrimitiveComponent Object Reference") (OtherBodyIndex :type Integer) (bFromSweep :type Boolean) (SweepResult :type "HitResult Structure (by ref)"))
  ;[1 1 1] execute every sequence
  (`|ExecutionSequence`
    (:`then_0`
      ;[1 1 1] if overlapped actor hast tag enemy and origin is player or actor has tag friend and origin is enemy take damage on target
      (if (`self.ActorHasTag` OtherActor "Enemy")
        (if (`KismetStringLibrary.EqualEqual_StrStr` (`self.Origin`) "Player")
          (bind _asbp_enemy (cast `/Game/character/enemy/BP_Enemy` OtherActor))
          (`/Game/character/enemy/BP_Enemy.TakeDamage` _asbp_enemy 35.0))
        (elif (`self.ActorHasTag` OtherActor "Friend")
          (if (`KismetStringLibrary.EqualEqual_StrStr` (`self.Origin`) "Enemy")
            (bind _asbp_friend (cast `/Game/character/friend/BP_Friend` OtherActor))
            (`/Game/character/friend/BP_Friend.TakeDamage` _asbp_friend 5.0)))))
    (:`then_1`
      ;[1 1 1] destroy actor
      (`self.K2_DestroyActor`))))

(fn `UserConstructionScript`)