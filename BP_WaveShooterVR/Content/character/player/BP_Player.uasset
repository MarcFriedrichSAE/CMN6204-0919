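; Player pawn for a shooter that creates the UI widget on BeginPlay and handles looking, walking and shooting.
; Each tick, look axes turn separate yaw and pitch roots, with pitch clamped and the skeletal mesh following yaw.
; Movement is a swept capsule offset along the yaw root's horizontal forward and right vectors, scaled by delta time.
; Shoot spawns a scaled-down BP_Bullet at BulletSpawn with camera rotation, tagging its Origin as Player.
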(event `self.ReceiveBeginPlay`
  ;[1 1 1] create ui widget
  (bind _returnvalue (`|CreateWidget` "/Game/ui/UMG_UI.UMG_UI_C"))
  (`UserWidget.AddToViewport` _returnvalue 0))

(event `self.ReceiveTick`
  (params (DeltaSeconds :type "Float (single-precision)"))
  ;[1 1 1] update every frame
  (`self.RotateCamera`)
  (`self.Move`))

(event `InputAction|Shoot`
  (params (Key :type "Key Structure"))
  ;[1 1 1] shoot bullet
  (:`Pressed`
    (bind _returnvalue (`|SpawnActorFromClass` "/Game/gameplay/BP_Bullet.BP_Bullet_C" (`KismetMathLibrary.MakeTransform` (`SceneComponent.K2_GetComponentLocation` (`self.BulletSpawn`)) (`SceneComponent.K2_GetComponentRotation` (`self.Camera`)) (0.1 0.1 0.1)) "Undefined" "OverrideRootScale" null null))
    (set `/Game/gameplay/BP_Bullet.Origin` "Player" _returnvalue)))

(fn `Move`
  (bind _camerayawroot (`self.CameraYawRoot`))
  (bind (_returnvalue_x _returnvalue_y) (`KismetMathLibrary.BreakVector` (`SceneComponent.GetForwardVector` _camerayawroot)))
  (bind (_returnvalue_x_2 _returnvalue_y_2) (`KismetMathLibrary.BreakVector` (`SceneComponent.GetRightVector` _camerayawroot)))
  ;[1 1 1] movement forward back and left right
  (`SceneComponent.K2_AddWorldOffset` (`self.Capsule`) (* (* (+ (* (`KismetMathLibrary.MakeVector` _returnvalue_x _returnvalue_y) (`self.GetInputAxisValue`)) (* (`KismetMathLibrary.MakeVector` _returnvalue_x_2 _returnvalue_y_2) (`self.GetInputAxisValue`))) (`self.MovementSpeed`)) (`GameplayStatics.GetWorldDeltaSeconds`)) true false))

(fn `RotateCamera`
  (bind _camerapitchroot (`self.CameraPitchRoot`))
  (bind (_relativerotation_roll _relativerotation_pitch _relativerotation_yaw) (`KismetMathLibrary.BreakRotator` (`SceneComponent.RelativeRotation` (`self.CameraYawRoot`))))
  (bind (_relativerotation_roll_2 _relativerotation_pitch_2) (`KismetMathLibrary.BreakRotator` (`SceneComponent.RelativeRotation` _camerapitchroot)))
  ;[1 1 1] rotate camera yaw
  (`SceneComponent.K2_AddLocalRotation` (`self.CameraYawRoot`) (`KismetMathLibrary.MakeRotator` 0.0 0.0 (* (`self.GetInputAxisValue`) (`self.RotationSpeed`) (`GameplayStatics.GetWorldDeltaSeconds`))) false false)
  ;[1 1 1] rotate camera pitch
  (`SceneComponent.K2_AddLocalRotation` (`self.CameraPitchRoot`) (`KismetMathLibrary.MakeRotator` 0.0 (* (`self.GetInputAxisValue`) (`self.RotationSpeed`) (`GameplayStatics.GetWorldDeltaSeconds`))) false false)
  ;[1 1 1] clamp camera pitch
  (`SceneComponent.K2_SetRelativeRotation` _camerapitchroot (`KismetMathLibrary.MakeRotator` 0.0 (`KismetMathLibrary.FMax` (`KismetMathLibrary.FMin` _relativerotation_pitch_2 45.0) -45.0)) false false)
  ;[1 1 1] rotate skeletal mesh
  (`SceneComponent.K2_SetRelativeRotation` (`self.SkeletalMesh`) (`KismetMathLibrary.MakeRotator` 0.0 0.0 (+ _relativerotation_yaw -90.0)) false false))

(fn `UserConstructionScript`)