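; Enemy actor that follows the nearest BP_Way spline toward the first "Friend"-tagged actor and shoots at it.
; BeginPlay caches that target's position and picks the closest path.
; Tick advances the capsule by swept moves, holding when blocked; once in range it permanently stops to fire BP_Bullets tagged with an "Enemy" origin.
; A health bar faces the player camera and scales with Health; TakeDamage destroys the actor at zero.
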(event `self.ReceiveBeginPlay`
  ;[1 1 1] get all friends and save position
  (bind _outactors (`GameplayStatics.GetAllActorsWithTag` "Friend"))
  (set `self.TargetPosition` (`self.K2_GetActorLocation` (`|GetArrayItem` _outactors)))
  ;[1 1 1] get player reference
  (bind _outactors_2 (`GameplayStatics.GetAllActorsOfClass` "/Game/character/player/BP_Player.BP_Player_C"))
  (set `self.Player` (`|GetArrayItem` _outactors_2))
  ;[1 1 1] get all way actor and check which one is the closest and save the reference
  (bind _outactors_3 (`GameplayStatics.GetAllActorsOfClass` "/Game/gameplay/BP_Way.BP_Way_C"))
  (for _array_element _outactors_3
    (bind _returnvalue (`KismetMathLibrary.VSizeSquared` (- (`self.K2_GetActorLocation` _array_element) (`self.K2_GetActorLocation`))))
    (if (<= _returnvalue (`self.PositionOnSpline`))
      (set `self.PositionOnSpline` _returnvalue)
      (set `self.Way` _array_element)))
  (set `self.PositionOnSpline` 0.0))

(event `self.ReceiveTick`
  (params (DeltaSeconds :type "Float (single-precision)"))
  (bind (_targetposition_x _targetposition_y) (`KismetMathLibrary.BreakVector` (`self.TargetPosition`)))
  (bind (_returnvalue_x _returnvalue_y) (`KismetMathLibrary.BreakVector` (`SceneComponent.K2_GetComponentLocation` (`self.Capsule`))))
  (bind (_returnvalue_roll _returnvalue_pitch _returnvalue_yaw) (`KismetMathLibrary.BreakRotator` (`SplineComponent.GetRotationAtDistanceAlongSpline` (`/Game/gameplay/BP_Way.Spline` (`self.Way`)) (`self.PositionOnSplineTemp`) "World")))
  ;[1 1 1] execute every sequence
  (`|ExecutionSequence`
    (:`then_0`
      ;[1 1 1] if friend is in shot range
      (if (`self.InShotRange`)
        ;[1 1 1] rotate capsule to target
        (`SceneComponent.K2_SetWorldRotation` (`self.Capsule`) (`KismetMathLibrary.FindLookAtRotation` (`KismetMathLibrary.MakeVector` _returnvalue_x _returnvalue_y) (`KismetMathLibrary.MakeVector` _targetposition_x _targetposition_y)) false false)
        ;[1 1 1] increase shot time and if higher than shot rate reset shot timer
        (bind _output_get (set `self.ShotTime` (+ (`self.ShotTime`) (`GameplayStatics.GetWorldDeltaSeconds`))))
        (if (>= _output_get (`self.SotRate`))
          (set `self.ShotTime` 0.0)
          ;[1 1 1] spawn bullet at bullet spawn and set origin of bullet to enemy
          (bind _returnvalue (`|SpawnActorFromClass` "/Game/gameplay/BP_Bullet.BP_Bullet_C" (`KismetMathLibrary.MakeTransform` (`SceneComponent.K2_GetComponentLocation` (`self.BulletSpawn`)) (`SceneComponent.K2_GetComponentRotation` (`self.Capsule`)) (0.1 0.1 0.1)) "Undefined" "OverrideRootScale" null null))
          (set `/Game/gameplay/BP_Bullet.Origin` "Enemy" _returnvalue))
        (else
          ;[1 1 1] if location is in shot range of target set in shot range true
          (if (< (`KismetMathLibrary.VSize` (- (`SceneComponent.K2_GetComponentLocation` (`self.Capsule`)) (`self.TargetPosition`))) (`self.ShotRange`))
            (set `self.InShotRange` true)
            (else
              ;[1 1 1] increase temp next position on spline by movement speed
              (set `self.PositionOnSplineTemp` (+ (`self.PositionOnSpline`) (* (`GameplayStatics.GetWorldDeltaSeconds`) (`self.MovementSpeed`))))
              ;[1 1 1] rotate capsule to next temp location on spline
              (`SceneComponent.K2_SetWorldRotation` (`self.Capsule`) (`KismetMathLibrary.MakeRotator` 0.0 0.0 _returnvalue_yaw) false false)
              ;[1 1 1] try to set location to next temp location on spline
              (bind _sweephitresult (`SceneComponent.K2_SetWorldLocation` (`self.Capsule`) (+ (`SplineComponent.GetLocationAtDistanceAlongSpline` (`/Game/gameplay/BP_Way.Spline` (`self.Way`)) (`self.PositionOnSplineTemp`) "World") (`KismetMathLibrary.MakeVector` 0.0 0.0 (`CapsuleComponent.CapsuleHalfHeight` (`self.Capsule`)))) true false))
              ;[1 1 1] if location set is working set current location on spline to temp location
              (if (`GameplayStatics.BreakHitResult` _sweephitresult)
                (set `self.PositionOnSplineTemp` (`self.PositionOnSpline`))
                (else
                  (set `self.PositionOnSpline` (`self.PositionOnSplineTemp`)))))))))
    (:`then_1`
      ;[1 1 1] if health bar valid rotate healthbar to player camera and set scale by health
      (`/Engine/EditorBlueprintResources/StandardMacros.IsValid` (`self.HealthBar`)
        (:`Is Valid`
          (`SceneComponent.K2_SetWorldRotation` (`self.HealthBarRoot`) (`KismetMathLibrary.FindLookAtRotation` (`SceneComponent.K2_GetComponentLocation` (`self.HealthBarRoot`)) (`SceneComponent.K2_GetComponentLocation` (`/Game/character/player/BP_Player.Camera` (`self.Player`)))) false false)
          (`SceneComponent.SetRelativeScale3D` (`self.HealthBar`) (`KismetMathLibrary.MakeVector` (* (`self.Health`) 0.01) 1.0 1.0)))))))

(fn `TakeDamage`
  (params (Damage :type "Float (double-precision)"))
  ;[1 1 1] decrease health and if lower than zero destroy actor
  (bind _output_get (set `self.Health` (- (`self.Health`) Damage)))
  (if (<= _output_get 0.0)
    (`self.K2_DestroyActor`)))

(fn `UserConstructionScript`)