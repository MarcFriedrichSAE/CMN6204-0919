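; Game mode that runs timed enemy waves from a queue of SWave structs.
; BeginPlay caches the locations of every BP_SpawnPoint.
; Tick counts down the first wave's start delay, then spawns its enemy type at random cached points on that wave's interval.
; Wave structs are rewritten in place as countdown and remaining-count state, and an exhausted wave is removed so the next begins counting down.
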(event `self.ReceiveBeginPlay`
  ;[1 1 1] check all spawn points and add location to spawn location array
  (bind _outactors (`GameplayStatics.GetAllActorsOfClass` "/Game/gameplay/BP_SpawnPoint.BP_SpawnPoint_C"))
  (for _array_element _outactors
    (`KismetArrayLibrary.Array_Add` (`self.SpawnPoints`) (`self.K2_GetActorLocation` _array_element))))

(event `self.ReceiveTick`
  (params (DeltaSeconds :type "Float (single-precision)"))
  (bind _waves (`self.Waves`))
  (bind _spawnpoints (`self.SpawnPoints`))
  (bind (_wavestarttime _enemytype _enemycount _spawntime) (break `/Game/utility/structs/S_Wave` (`|GetArrayItem` (`self.Waves`))))
  (bind (_wavestarttime_2 _enemytype_2 _enemycount_2 _spawntime_2) (break `/Game/utility/structs/S_Wave` (`|GetArrayItem` _waves)))
  ;[1 1 1] if waves length higher than zero
  (if (> (`KismetArrayLibrary.Array_Length` (`self.Waves`)) 0)
    ;[1 1 1] if first waves time to start wave under zero
    (if (<= (`.WaveStartTime_11_C5CB2EB34FBD516CD619B2864C40C335` (break `/Game/utility/structs/S_Wave` (`|GetArrayItem` (`self.Waves`)))) 0.0)
      ;[1 1 1] increase spawn time and if higher than current wave enemy spawn time reset spawn time
      (bind _output_get (set `self.SpawnTime` (+ (`self.SpawnTime`) (`GameplayStatics.GetWorldDeltaSeconds`))))
      (if (>= _output_get (`.SpawnTime_5_0464E893466E2A3EE95358B649C5EBA3` (break `/Game/utility/structs/S_Wave` (`|GetArrayItem` (`self.Waves`)))))
        (set `self.SpawnTime` 0.0)
        ;[1 1 1] decrease enemy count of current wave
        (`KismetArrayLibrary.Array_Set` _waves 0 (make `/Game/utility/structs/S_Wave` _wavestarttime_2 _enemytype_2 (- _enemycount_2 1) _spawntime_2))
        ;[1 1 1] spawn enemy at random spawn location
        (`|SpawnActorFromClass` (`.EnemyType_12_9A38791E4101A36B3C98839A056D2829` (break `/Game/utility/structs/S_Wave` (`|GetArrayItem` (`self.Waves`)))) (`KismetMathLibrary.MakeTransform` (`|GetArrayItem` _spawnpoints (`KismetMathLibrary.RandomIntegerInRange` 0 (- (`KismetArrayLibrary.Array_Length` _spawnpoints) 1)))) "Undefined" "OverrideRootScale" null null)
        ;[1 1 1] if enemy count is lower than zero remove first wave
        (if (<= (`.EnemyCount_2_5299A1AD409E709A7CEFC684A39938B3` (break `/Game/utility/structs/S_Wave` (`|GetArrayItem` (`self.Waves`)))) 0)
          (`KismetArrayLibrary.Array_Remove` (`self.Waves`))))
      (else
        ;[1 1 1] decrease wave spawn timer
        (`KismetArrayLibrary.Array_Set` (`self.Waves`) 0 (make `/Game/utility/structs/S_Wave` (- _wavestarttime (`GameplayStatics.GetWorldDeltaSeconds`)) _enemytype _enemycount _spawntime))))))

(fn `UserConstructionScript`)