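; BP_Player is the player Blueprint, handling movement, look rotation, shooting and teleporting.
; Tick passes movement and look values from getter functions into Move and Rotate every frame.
; Pressing Fire calls Shoot, while Teleport uses press-and-release: pressing calls ShowTeleport and releasing calls Teleport.
; The graph only routes input to these functions, whose logic is not defined here, and the construction script is empty.
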(event `self.ReceiveTick`
  (params (DeltaSeconds :type "Float (single-precision)"))
  ;[1 1 1] move and rotate player
  (`self.Move` (`self.GetInputAxisValue`) (`self.GetInputAxisValue`))
  (`self.Rotate` (`self.GetInputAxisValue`) (`self.GetInputAxisValue`)))

(event `InputAction|Fire`
  (params (Key :type "Key Structure"))
  ;[1 1 1] shoot bullet
  (:`Pressed`
    (`self.Shoot`)))

(event `InputAction|Teleport`
  (params (Key :type "Key Structure"))
  ;[1 1 1] teleport
  (:`Pressed`
    (`self.ShowTeleport`))
  (:`Released`
    (`self.Teleport`)))

(fn `UserConstructionScript`)